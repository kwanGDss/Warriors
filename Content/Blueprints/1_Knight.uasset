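; Knight character Blueprint with stamina, rolling and melee combo attacks, set against the Viking as its enemy.
; It creates a status bar widget on BeginPlay and updates health and stamina bars each Tick.
; Running drains stamina, rolling spends a chunk on Space, and stamina regenerates otherwise.
; Left click plays the attack montage and buffers further clicks, which ResetCombo uses to continue or stop the combo, while AttackEnd clears attack state.
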(event EventBeginPlay
  (bind _returnvalue (UserInterface|CreateWidget "/Game/UI/UI_CharacterStatusBar.UI_CharacterStatusBar_C"))
  (bind _output_get (Variables|Default|SetCharacterStatusBar _returnvalue))
  (UserInterface|Viewport|AddtoViewport _output_get 0)
  (Variables|Default|SetStamina 1.0)
  (Variables|Default|SetHealth 1.0))

(event Collision|EventActorBeginOverlap
  (params (OtherActor :type Actor%20Object%20Reference)))

(event EventTick
  (params (DeltaSeconds :type Float%20%28single-precision%29))
  (|StaminaSystem)
  (Progress|SetPercent (Variables|/Game/UI/UI_CharacterStatusBar.UI_CharacterStatusBar_C|GetHealthBar (Variables|Default|GetCharacterStatusBar)) (Variables|Default|GetHealth)))

(event Input|MouseEvents|LeftMouseButton
  (params (Key :type Key%20Structure :default "None"))
  (:Pressed
    (|AttackSystem)))

(fn ConstructionScript
  (Variables|Default|SetStamina 1.0)
  (Class|WarriorsCharacter|SetEnemyCharacter "/Game/Blueprints/2_Viking.2_Viking_C"))

(event Input|KeyboardEvents|SpaceBar
  (params (Key :type Key%20Structure :default "None"))
  (:Pressed
    (if (not (Variables|Default|GetbIsRolling))
      (if (< 0.25 (Variables|Default|GetStamina))
        (Variables|Default|SetRollStartedTime (Utilities|Time|GetTimeSeconds))
        (Variables|Default|SetStamina (- (Variables|Default|GetStamina) 0.25))
        (Variables|Default|SetbIsRolling true)))))

(event Custom|AttackEnd
  (Variables|Default|SetSaveAttack false)
  (Variables|Default|SetIsAttacking false)
  (return))

(event Custom|ResetCombo
  (if (Variables|Default|GetSaveAttack)
    (Variables|Default|SetSaveAttack false)
    (else
      (Variables|Default|SetSaveAttack false)
      (Variables|Default|SetIsAttacking false)
      (Animation|StopAnimMontage "/Game/Animations/AM_Knight_Attack.AM_Knight_Attack")))
  (return))