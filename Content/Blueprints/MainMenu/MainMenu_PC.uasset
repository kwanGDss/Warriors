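; Main menu player controller that loads the local Steam profile and friends on BeginPlay, only when the Steam subsystem is present.
; It puts the player's name and avatar into PlayerInfo, saves it and notifies the menu through GameInstance messages, continuing even if the avatar fetch fails.
; It then fetches the friends list, forwarding only friends in the Away state, with their avatars, to the GameInstance.
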(event EventBeginPlay
  (bind _returnvalue (Game|GetGameInstance))
  (if (Class|AdvancedSessionsLibrary|HasOnlineSubsystem "STEAM")
    (Variables|Default|SetPlayerName (Utilities|Text|ToText(String) (Class|AdvancedSessionsLibrary|GetPlayerName self)))
    (bind _returnvalue_2 (Class|AdvancedSteamFriendsLibrary|GetSteamFriendAvatar (Class|AdvancedSessionsLibrary|GetUniqueNetID self) "SteamAvatar_Medium")
      (:OnSuccess
        _)
      (:OnFailure
        _))
    (bind _structout (Utilities|Struct|SetmembersinPlayerInfo (Variables|Default|GetPlayerInfo) (Variables|Default|GetPlayerName) _returnvalue_2))
    (Class|GameInfoInstanceBPI|SavePlayerInfo(Message) _returnvalue _structout)
    (Class|GameInfoInstanceBPI|MainMenuPlayerInfo(Message) _returnvalue)
    (bind _results (|GetandStoreFriendsList self)
      (:OnSuccess
        (for _array_element _results
          (if (Utilities|Enum|Equal(Enum) (.OnlineState (Utilities|Struct|BreakBPFriendInfo _array_element)) "Away")
            (bind _returnvalue_3 (Class|AdvancedSteamFriendsLibrary|GetSteamFriendAvatar (.UniqueNetId (Utilities|Struct|BreakBPFriendInfo _array_element)) "SteamAvatar_Medium")
              (:OnSuccess
                (Class|GameInfoInstanceBPI|UpdateFriendList(Message) (Game|GetGameInstance) _array_element _returnvalue_3)))))))))

(fn ConstructionScript)