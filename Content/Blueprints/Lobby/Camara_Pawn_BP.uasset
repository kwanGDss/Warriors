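; Lobby camera pawn that passes itself to the lobby player controller on BeginPlay and handles movement and look input.
; BeginPlay also runs two one-shot sequences with hardcoded conditions, each applying a single interpolation step rather than updating on Tick.
; These ease control and actor rotation toward a lock-on direction derived from the pawn's normalized world location, and adjust spring arm length.
; Movement follows control yaw, while roll axes are only stored.
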(event Custom|Sequence_0
  ;[1 1 1] Sequence 0
  (if true
    (bind _output_get (Variables|Default|SetLockOnDirection (Math|Vector|Normalize (Transformation|GetActorLocation) 0.1)))
    (bind _output_get_2 (Variables|Default|SetLockOnRotation (Math|Rotator|MakeRotator (.Roll (Math|Rotator|BreakRotator (Math|Rotator|MakeRotfromX _output_get))) (- (.Pitch (Math|Rotator|BreakRotator (Math|Rotator|MakeRotfromX _output_get))) 1e+01) (.Yaw (Math|Rotator|BreakRotator (Math|Rotator|MakeRotfromX _output_get))))))
    (Variables|Default|SetLockOnInterpolationRotation (Math|Interpolation|RInterpTo (Pawn|GetControlRotation (Pawn|GetController) :!class /Script/Engine.Controller) _output_get_2 (Utilities|Time|GetWorldDeltaSeconds) 0.0))
    (bind _output_get_3 (Variables|Default|SetLockOnRotation (Math|Rotator|MakeRotator (.Roll (Math|Rotator|BreakRotator _output_get_2)) 0.0 (.Yaw (Math|Rotator|BreakRotator _output_get_2)))))
    (if true
      (Transformation|SetActorRotation (Math|Interpolation|RInterpTo (Transformation|GetActorRotation) _output_get_3 (Utilities|Time|GetWorldDeltaSeconds) 0.0)))
    (Pawn|SetControlRotation (Pawn|GetController) (Variables|Default|GetLockOnInterpolationRotation))))

(event Custom|Sequence_1
  (bind _returnvalue (Utilities|Time|GetWorldDeltaSeconds))
  (bind _cameraboom (Variables|Default|GetCameraBoom))
  ;[1 1 1] Sequence 1
  (if true
    (Variables|/Script/Engine.SpringArmComponent|SetTargetArmLength _cameraboom (Math|Interpolation|FInterpTo (Variables|/Script/Engine.SpringArmComponent|GetTargetArmLength _cameraboom) 4e+02 _returnvalue 0.0))
    (else
      (Variables|/Script/Engine.SpringArmComponent|SetTargetArmLength _cameraboom (Math|Interpolation|FInterpTo (Variables|/Script/Engine.SpringArmComponent|GetTargetArmLength _cameraboom) 3e+02 _returnvalue 1e+01)))))

(event EventBeginPlay
  (bind _lobbypc (Class|LobbyPCBPI|LobbyPCRef(Message) (Game|GetPlayerController 0)))
  (Default|GetCameraObj _lobbypc)
  (Default|GetPawn _lobbypc self)
  (CallFunction|Sequence0)
  (CallFunction|Sequence1))

(event Input|AxisEvents|InputAxisRollForward
  (params (AxisValue :type Float%20%28single-precision%29))
  (Variables|Default|SetMoveForwardAxis AxisValue))

(event Input|AxisEvents|InputAxisRollRight
  (params (AxisValue :type Float%20%28single-precision%29))
  (Variables|Default|SetMoveRightAxis AxisValue))

(event Input|AxisEvents|InputAxisLookUp
  (params (AxisValue :type Float%20%28single-precision%29))
  (Pawn|Input|AddControllerPitchInput AxisValue))

(event Input|AxisEvents|InputAxisTurn
  (params (AxisValue :type Float%20%28single-precision%29))
  (Pawn|Input|AddControllerYawInput AxisValue))

(event Input|AxisEvents|InputAxisMoveForward
  (params (AxisValue :type Float%20%28single-precision%29))
  (Pawn|Input|AddMovementInput (Math|Vector|GetForwardVector (Math|Rotator|MakeRotator 0.0 0.0 (.Yaw (Math|Rotator|BreakRotator (Pawn|GetControlRotation :!class /Script/Engine.Pawn))))) AxisValue false))

(event Input|AxisEvents|InputAxisMoveRight
  (params (AxisValue :type Float%20%28single-precision%29))
  (Pawn|Input|AddMovementInput (Math|Vector|GetRightVector (Math|Rotator|MakeRotator 0.0 0.0 (.Yaw (Math|Rotator|BreakRotator (Pawn|GetControlRotation :!class /Script/Engine.Pawn))))) AxisValue false))

(fn ConstructionScript)