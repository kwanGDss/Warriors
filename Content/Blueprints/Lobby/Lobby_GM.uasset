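; Lobby game mode that manages joining players, map settings, character choice, kicking and match launch for a multiplayer lobby.
; On login it initializes each lobby PlayerController from GameInstance server data and possesses a Knight at a random PlayerStart.
; It loops over stored controllers to push settings, player lists and counts, and derives CanStart from character picks.
; Launch shows loading screens, then server-travels to the hardcoded Warriors map, regardless of selected map.
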(event Custom|SwapCharacter
  (params (PlayerController :type Player%20Controller%20Object%20Reference) (Character :type Character%20Class%20Reference) (ChangeStatus :type Boolean))
  (bind _returnvalue (Pawn|GetControlledPawn PlayerController))
  (bind _spawnpoint (Variables|ServerSetting|GetSpawnPoint))
  ;[1 1 1] Swap Current Character with Select Charater
  (if (not ChangeStatus)
    (Utilities|IsValid _returnvalue
      (:Is%20Valid
        (Actor|DestroyActor _returnvalue))
      (:Is%20Not%20Valid
        _))
    (bind _returnvalue_2 (Game|SpawnActorfromClass Character (Transformation|GetActorTransform (Utilities|Array|Get(acopy) _spawnpoint (Math|Random|RandomIntegerinRange 0 (- (Utilities|Array|Length _spawnpoint) 1)))) "AlwaysSpawn" 0 0))
    (Pawn|Possess PlayerController _returnvalue_2)))

(event Custom|EveryoneUpdate
  (bind _allplayercontroller (Variables|ServerSetting|GetAllPlayerController))
  ;[1 1 1] Update Connected Player to Lobby Info
  (bind _output_get (Variables|ServerSetting|SetCurrentPlayer (Utilities|Array|Length (Variables|ServerSetting|GetAllPlayerController))))
  (if (> _output_get 0)
    (Utilities|Array|Clear (Variables|ServerSetting|GetConnectedPlayer))
    (for _array_element _allplayercontroller
      (bind _lobbypc (Class|LobbyPCBPI|LobbyPCRef(Message) _array_element))
      (Utilities|Array|Add (Variables|ServerSetting|GetConnectedPlayer) (Variables|/Game/Blueprints/Lobby/Lobby_PC.Lobby_PC_C|GetPlayerSetting _lobbypc))
      (Default|UpdateNumberofPlayer _lobbypc (Variables|ServerSetting|GetCurrentPlayer) (Variables|ServerSetting|GetMax_Player)))
    (for _array_element_2 _allplayercontroller
      (bind _lobbypc_2 (Class|LobbyPCBPI|LobbyPCRef(Message) _array_element_2))
      (Default|AddPlayerInfo _lobbypc_2 (Variables|ServerSetting|GetConnectedPlayer))
      (CallFunction|AddtoKickList))
    (bind _array_element_3 (Utilities|Array|ForEachLoopwithBreak (Variables|ServerSetting|GetConnectedPlayer))
      (:LoopBody
        (if (== (.MyPlayerCharacter (Utilities|Struct|BreakPlayerInfo _array_element_3)) "/Game/Blueprints/Characters/0_Base.0_Base_C")
          (Variables|ServerSetting|SetCanStart false)
          (CallFunction|CanNotStartGame)
          (else
            (Variables|ServerSetting|SetCanStart true)))))))

(event Custom|LaunchTheGame
  ;[1 1 1] Launch Game by Map Selection
  (Development|ExecuteConsoleCommand "servertravel /Game/Maps/Warriors" (Game|GetPlayerController 0))
  (for _array_element (Variables|ServerSetting|GetAllPlayerController)
    (bind _lobbypc (Class|LobbyPCBPI|LobbyPCRef(Message) _array_element))
    (Default|DestroyLoadingScreen _lobbypc)))

(event Custom|SpawnPlayer
  (params (PlayerController :type Player%20Controller%20Object%20Reference))
  (bind _returnvalue (Pawn|GetControlledPawn PlayerController))
  (bind _spawnpoint (Variables|ServerSetting|GetSpawnPoint))
  ;[1 1 1] Spawn Player with Base Character when Enter and Notify Everyone to Update Lobby Status
  (Utilities|IsValid _returnvalue
    (:Is%20Valid
      (Actor|DestroyActor _returnvalue))
    (:Is%20Not%20Valid
      _))
  (bind _returnvalue_2 (Game|SpawnActorfromClass "/Game/Blueprints/Characters/1_Knight.1_Knight_C" (Transformation|GetActorTransform (Utilities|Array|Get(acopy) _spawnpoint (Math|Random|RandomIntegerinRange 0 (- (Utilities|Array|Length _spawnpoint) 1)))) "Undefined" 0 0))
  (Pawn|Possess PlayerController _returnvalue_2)
  (CallFunction|EveryoneUpdate))

(event Custom|AddToKickList
  ;[1 1 1] Add Player Kicked List when Player Connecting
  (bind _lobbypc (Class|LobbyPCBPI|LobbyPCRef(Message) (Game|GetPlayerController 0)))
  (bind _lobbymenuwb (Variables|/Game/Blueprints/Lobby/Lobby_PC.Lobby_PC_C|GetLobbyMenuWB _lobbypc)
    (:then
      (if (Widget|IsVisible (Variables|/Game/UI/Lobby/LobbyMenu.LobbyMenu_C|GetGameSettings _lobbymenuwb))
        (Default|FillPlayeronWindow (Variables|/Game/UI/Lobby/LobbyMenu.LobbyMenu_C|GetGameSettings _lobbymenuwb))))
    (:else)))

(event Custom|CanNotStartGame
  ;[1 1 1] Update Connected Player to Lobby Info
  (Utilities|Array|ForEachLoopwithBreak (Variables|ServerSetting|GetConnectedPlayer)) ; enters at Break
)

(event Custom|ServerUpdateGameSetting
  (params (MapImage :type Texture%202D%20Object%20Reference) (MapName :type Text) (MapTime :type Text) (MapID :type Integer))
  ;[1 1 1] Server Has Change, Notify Everyone to Update Lobby Info
  (Variables|ServerSetting|SetGM_MapImage MapImage)
  (Variables|ServerSetting|SetGM_MapName MapName)
  (Variables|ServerSetting|SetGM_MapTime MapTime)
  (Variables|ServerSetting|SetGM_MapID MapID)
  (for _array_element (Variables|ServerSetting|GetAllPlayerController)
    (bind _lobbypc (Class|LobbyPCBPI|LobbyPCRef(Message) _array_element))
    (Default|UpdateLobbySetting _lobbypc (Variables|ServerSetting|GetGM_MapImage) (Variables|ServerSetting|GetGM_MapName) (Variables|ServerSetting|GetGM_MapTime))))

(event Custom|CanKick
  (params (PlayerID :type Integer))
  ;[1 1 1] Kick opposite Player in Lobby
  (bind _lobbypc (Class|LobbyPCBPI|LobbyPCRef(Message) (Utilities|Array|Get(acopy) (Variables|ServerSetting|GetAllPlayerController) PlayerID)))
  (Default|Kicked _lobbypc))

(event Custom|StartLoadingScreen
  ;[1 1 1] Start Loading Screen each Client
  (for _array_element (Variables|ServerSetting|GetAllPlayerController)
    (bind _lobbypc (Class|LobbyPCBPI|LobbyPCRef(Message) _array_element))
    (Default|ShowLoadingScreen _lobbypc))
  (CallFunction|LaunchtheGame))

(event EventPostLogin
  (params (NewPlayer :type Player%20Controller%20Object%20Reference))
  ;[1 1 1] Init Setting when Post Log-in and Handle Lobby Set up on Player Controller & Spawn Player
  (Variables|Default|SetConnectingPlayer NewPlayer)
  (Utilities|Array|Add (Variables|ServerSetting|GetAllPlayerController) NewPlayer)
  (bind _outactors (Actor|GetAllActorsOfClass "/Script/Engine.PlayerStart"))
  (Variables|ServerSetting|SetSpawnPoint _outactors)
  (bind _gameinfoinstance (Class|GameInfoInstanceBPI|GameInstanceRef(Message) (Game|GetGameInstance)))
  (Variables|ServerSetting|SetServer_Name (Variables|/Game/Blueprints/AllLevels/GameInfoInstance.GameInfoInstance_C|GetServerName _gameinfoinstance))
  (Variables|ServerSetting|SetMax_Player (Variables|/Game/Blueprints/AllLevels/GameInfoInstance.GameInfoInstance_C|GetMaxPlayer _gameinfoinstance))
  (bind _lobbypc (Class|LobbyPCBPI|LobbyPCRef(Message) NewPlayer))
  (bind _output_get (Variables|ServerSetting|SetLobby%20PC _lobbypc))
  (Default|InitSetup _output_get)
  (Default|SetupLobbyMenu (Variables|ServerSetting|GetLobby%20PC) (Variables|ServerSetting|GetServer_Name))
  (Default|UpdateLobbySetting (Variables|ServerSetting|GetLobby%20PC) (Variables|ServerSetting|GetGM_MapImage) (Variables|ServerSetting|GetGM_MapName) (Variables|ServerSetting|GetGM_MapTime))
  (CallFunction|SpawnPlayer NewPlayer))

(event EventOnLogout
  (params (ExitingController :type Controller%20Object%20Reference))
  ;[1 1 1] OnLogout Event Removes Player Controller
  (bind (_array_element _array_index) (Utilities|Array|ForEachLoopwithBreak (Variables|ServerSetting|GetAllPlayerController) :!label _label)
    (:LoopBody
      (if (== ExitingController _array_element)
        (goto _label Break)))
    (:Completed
      (Utilities|Array|RemoveIndex (Variables|ServerSetting|GetAllPlayerController) _array_index)
      (Utilities|Array|RemoveIndex (Variables|ServerSetting|GetConnectedPlayer) _array_index)
      (CallFunction|EveryoneUpdate))))

(fn ConstructionScript)

(fn LobbyGMRef
  (return self))