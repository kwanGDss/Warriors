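; Playable Knight character with stamina-gated melee combat: running, rolling, attacks, running attack, parry, guard and attack-stance toggles.
; Input events play montages, while animation-driven events buffer a combo follow-up, track stance transitions and toggle sword capsule collision for damage.
; Tick drains or regenerates stamina and pushes it with health to the player controller's HUD message interface.
; Construction sets the Viking as enemy, but the code notifying it of parries is disconnected.
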(event OnComponentBeginOverlap(SwordCapsuleComponent)
  (params (OverlappedComponent :type Primitive%20Component%20Object%20Reference) (OtherActor :type Actor%20Object%20Reference) (OtherComp :type Primitive%20Component%20Object%20Reference) (OtherBodyIndex :type Integer) (bFromSweep :type Boolean) (SweepResult :type Hit%20Result%20Structure%20%28by%20ref%29))
  (if (not (== OtherActor self))
    (Game|Damage|ApplyDamage OtherActor 0.2 0 self)
    (Collision|SetCollisionEnabled (Variables|Default|GetSwordCapsuleComponent) "NoCollision")))

(event Custom|OnCollStart_Attack
  (Collision|SetCollisionEnabled (Variables|Default|GetSwordCapsuleComponent) "QueryAndPhysics")
  (Variables|Default|SetStamina (- (Variables|Default|GetStamina) 0.15)))

(event Custom|OnCollEnd_Attack
  (Collision|SetCollisionEnabled (Variables|Default|GetSwordCapsuleComponent) "NoCollision"))

(event Custom|AttackState_Loop_Lefted
  (Variables|Default|Set%20IsPlayedAttackStateSwitch true))

(event Custom|AttackEnd
  (Variables|Default|SetSaveAttack false)
  (Variables|Default|SetIsAttacking false))

(event Custom|Play%20Attack
  (Animation|PlayAnimMontage "/Game/Animations/AM_Knight_Attack_1.AM_Knight_Attack_1" 1.0 "None"))

(event Custom|Play%20Combo%20Attack%201
  (Animation|PlayAnimMontage "/Game/Animations/AM_Knight_Attack.AM_Knight_Attack" 1.0 "ComboAttack_1"))

(event Custom|Stop%20Attack
  (Animation|StopAnimMontage "/Game/Animations/AM_Knight_Attack.AM_Knight_Attack"))

(event Custom|Play%20RunAttack
  (Animation|PlayAnimMontage "/Game/Animations/AM_Knight_RunAttack.AM_Knight_RunAttack" 1.0 "None")
  (Variables|Default|SetIsAttackState true))

(event Custom|Play%20Parring
  (Animation|PlayAnimMontage "/Game/Animations/AM_Knight_Parrying.AM_Knight_Parrying" 1.0 "None")
  (Variables|Default|SetIsAttackState true))

(event Custom|Parrying_Start
  (Variables|Default|SetCanParry true)
  (Collision|SetCollisionEnabled (Variables|Default|GetSwordCapsuleComponent) "QueryAndPhysics"))

(event Custom|Parrying_End
  (Variables|Default|SetCanParry false)
  (Collision|SetCollisionEnabled (Variables|Default|GetSwordCapsuleComponent) "NoCollision"))

(event Custom|FindCollSwordEventBreakLoop
  (Utilities|Array|ForEachLoopwithBreak (Actor|GetComponentsByClass (stale OnComponentBeginOverlap(SwordCapsuleComponent) OtherActor) "/Script/Engine.CapsuleComponent")) ; enters at Break
)

(event Custom|AttackState_Start_Entered
  (Variables|Default|Set%20IsPlayedAttackStateSwitch true))

(event Custom|AttackState_Loop_Entered
  (Variables|Default|Set%20IsPlayedAttackStateSwitch false))

(event Custom|ResetCombo
  (bind _mesh (Variables|Character|GetMesh))
  (bind _returnvalue (Components|SkeletalMesh|GetAnimInstance _mesh))
  (bind _returnvalue_2 (Animation|Montage|MontageIsPlaying _returnvalue "/Game/Animations/AM_Knight_Attack_1.AM_Knight_Attack_1"))
  (if (Variables|Default|GetSaveAttack)
    (Variables|Default|SetSaveAttack false)
    (if _returnvalue_2
      (CallFunction|PlayComboAttack1))
    (else
      (Variables|Default|SetSaveAttack false)
      (Variables|Default|SetIsAttacking false)
      (if (not _returnvalue_2)
        (CallFunction|StopAttack)))))

(event Custom|Roll_FullBlend
  (Variables|Default|SetIsAttackState true))

(event Custom|Play%20Roll
  (Animation|PlayAnimMontage "/Game/Animations/AM_Knight_Roll.AM_Knight_Roll" 1.0 "None")
  (if (not (Variables|Default|GetbIsLockOnState))
    (Class|WarriorsCharacter|Lockon)))

(event Custom|AttackState_End_Lefted
  (Variables|Default|Set%20IsPlayedAttackStateSwitch false))

(event EventTick
  (params (DeltaSeconds :type Float%20%28single-precision%29))
  (Utilities|FlowControl|Sequence
    (:then_0
      (if (and (not (Class|AnimInstance|IsAnyMontagePlaying (Components|SkeletalMesh|GetAnimInstance (Variables|Character|GetMesh)))) (Variables|Default|GetbIsRunning))
        (if (> (Variables|Default|GetStamina) 0.0)
          (Variables|Default|SetStamina (- (Variables|Default|GetStamina) (* (Utilities|Time|GetWorldDeltaSeconds) 0.1))))))
    (:then_1
      (if (Class|KismetMathLibrary|XORBoolean (Math|Boolean|NORBoolean (Variables|Default|GetbIsRunning) (Variables|Default|GetbIsRolling)) (Variables|Default|GetIsAttacking))
        (if (> 1.0 (Variables|Default|GetStamina))
          (Variables|Default|SetStamina (+ (Variables|Default|GetStamina) (* (Utilities|Time|GetWorldDeltaSeconds) 0.2))))))
    (:then_2
      (if (Variables|Default|GetbIsRolling)
        (Variables|Default|SetbIsRunning false)))
    (:then_3
      (bind _gameplay_gm_ref (Class|GameplayGMBPI|GameplayGMRef(Message) (Game|GetPlayerController 0)))
      (Default|SetStamia _gameplay_gm_ref (Variables|Default|GetStamina))
      (Default|SetHealth _gameplay_gm_ref (Variables|Default|GetHealth))
      (if (Variables|Default|GetbIsLockOnState)
        (Variables|Default|SetIsAttackState true)))))

(event Game|Damage|EventAnyDamage
  (params (Damage :type Float%20%28single-precision%29) (DamageType :type Damage%20Type%20Object%20Reference) (InstigatedBy :type Controller%20Object%20Reference) (DamageCauser :type Actor%20Object%20Reference))
  (Variables|Default|SetHealth (- (Variables|Default|GetHealth) Damage)))

(event Input|MouseEvents|LeftMouseButton
  (params (Key :type Key%20Structure :default "None"))
  (bind _stamina (Variables|Default|GetStamina))
  (bind _returnvalue (< 0.1 _stamina))
  (:Pressed
    (if (Variables|Default|GetIsAttackState)
      (if _returnvalue
        (if (Math|Boolean|NORBoolean (Variables|Default|GetbIsRolling) (Variables|Default|Get%20IsPlayedAttackStateSwitch))
          (if (Variables|Default|GetIsAttacking)
            (Variables|Default|SetSaveAttack true)
            (else
              (Variables|Default|SetIsAttacking true)
              (CallFunction|PlayAttack)))))
      (elif (Variables|Default|GetbIsRunning)
        (if _returnvalue
          (CallFunction|PlayRunAttack))
        (else
          (Variables|Default|SetIsAttackState true)
          (if (not (Variables|Default|GetbIsLockOnState))
            (Class|WarriorsCharacter|Lockon)))))))

(event Input|KeyboardEvents|Tab
  (params (Key :type Key%20Structure :default "None")))

(event Input|KeyboardEvents|Q
  (params (Key :type Key%20Structure :default "None"))
  (:Pressed
    (if true
      (if (Variables|Default|GetIsGuard)
        (Variables|Default|SetIsGuard false)
        (else
          (Variables|Default|SetIsGuard true))))))

(event Input|KeyboardEvents|C
  (params (Key :type Key%20Structure :default "None"))
  (:Pressed
    (if (not (Variables|Default|GetbIsRolling))
      (if (not (Class|AnimInstance|IsAnyMontagePlaying (Components|SkeletalMesh|GetAnimInstance (Variables|Character|GetMesh))))
        (Variables|Default|SetStamina (Math|Float|Clamp(Float) (- (Variables|Default|GetStamina) 0.4)))
        (CallFunction|PlayParring)))))

(event Input|KeyboardEvents|R
  (params (Key :type Key%20Structure :default "None"))
  (:Pressed
    (if (Variables|Default|GetIsAttackState)
      (Variables|Default|SetIsAttackState false)
      (else
        (Variables|Default|SetIsAttackState true)))))

(event Input|KeyboardEvents|SpaceBar
  (params (Key :type Key%20Structure :default "None"))
  (:Pressed
    (if (Math|Boolean|NORBoolean (Class|AnimInstance|IsAnyMontagePlaying (Components|SkeletalMesh|GetAnimInstance (Variables|Character|GetMesh))) (Variables|Default|GetbIsRolling))
      (if (< 0.2 (Variables|Default|GetStamina))
        (Variables|Default|SetRollStartedTime (Utilities|Time|GetTimeSeconds))
        (Variables|Default|SetStamina (- (Variables|Default|GetStamina) 0.2))
        (Variables|Default|SetbIsRolling true)
        (if (Variables|Default|GetbIsLockOnState)
          (Transformation|SetActorRotation (Math|Conversions|RotationFromXVector (Math|Vector|Normalize (+ (* (Transformation|GetActorRightVector) (Variables|Default|GetMoveRightAxis)) (* (Transformation|GetActorForwardVector) (Variables|Default|GetMoveForwardAxis)))))))
        (CallFunction|PlayRoll)))))

(fn ConstructionScript
  (Variables|Default|SetHealth 1.0)
  (Variables|Default|SetStamina 1.0)
  (Class|WarriorsCharacter|SetEnemyCharacter "/Game/Blueprints/Characters/2_Viking.2_Viking_C")
  (Variables|/Script/Engine.SpringArmComponent|SetbDoCollisionTest (Variables|Default|GetCameraBoom) false))

(fn BPIsMoveSituation
  (if (or (Variables|Default|GetIsAttacking) (Variables|Default|Get%20IsPlayedAttackStateSwitch))
    (return false)
    (else
      (return true))))