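; Third-person player character with lock-on to a WarriorsCharacter found at construction, plus standard movement and look input.
; Tick runs sequenced custom events that snap actor and control rotation toward the enemy, set boom length and force walking speed.
; Much is stubbed: several events are empty, branches use constant conditions, and BP_IsMoveSituation always returns false.
; Roll axes are stored, but the energy-costing directional roll logic is never executed.
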(event Custom|Sequence_0
  ;[1 1 1] Sequence 0
  (if (Variables|Default|GetIsLockOnState)
    (bind _output_get (Variables|Default|SetLockOnDirection (Math|Vector|Normalize (- (Transformation|GetActorLocation (Variables|Default|GetEnemyCharacter)) (Transformation|GetActorLocation)) 0.1)))
    (bind _output_get_2 (Variables|Default|SetLockOnRotation (Math|Rotator|MakeRotator (.Roll (Math|Rotator|BreakRotator (Math|Rotator|MakeRotfromX _output_get))) (- (.Pitch (Math|Rotator|BreakRotator (Math|Rotator|MakeRotfromX _output_get))) 1e+01) (.Yaw (Math|Rotator|BreakRotator (Math|Rotator|MakeRotfromX _output_get))))))
    (Variables|Default|SetLockOnInterpolationRotation (Math|Interpolation|RInterpTo (Pawn|GetControlRotation (Pawn|GetController) :!class /Script/Engine.Controller) _output_get_2 (Utilities|Time|GetWorldDeltaSeconds) 0.0))
    (bind _output_get_3 (Variables|Default|SetLockOnRotation (Math|Rotator|MakeRotator (.Roll (Math|Rotator|BreakRotator _output_get_2)) 0.0 (.Yaw (Math|Rotator|BreakRotator _output_get_2)))))
    (if true
      (Transformation|SetActorRotation (Math|Interpolation|RInterpTo (Transformation|GetActorRotation) _output_get_3 (Utilities|Time|GetWorldDeltaSeconds) 0.0)))
    (Pawn|SetControlRotation (Pawn|GetController) (Variables|Default|GetLockOnInterpolationRotation))))

(event Custom|Sequence_1
  (bind _returnvalue (Utilities|Time|GetWorldDeltaSeconds))
  (bind _cameraboom (Variables|Default|GetCameraBoom))
  ;[1 1 1] Sequence 1
  (if true
    (Variables|/Script/Engine.SpringArmComponent|SetTargetArmLength _cameraboom (Math|Interpolation|FInterpTo (Variables|/Script/Engine.SpringArmComponent|GetTargetArmLength (Variables|Default|GetCameraBoom)) 4e+02 _returnvalue 0.0))
    (else
      (Variables|/Script/Engine.SpringArmComponent|SetTargetArmLength _cameraboom (Math|Interpolation|FInterpTo (Variables|/Script/Engine.SpringArmComponent|GetTargetArmLength (Variables|Default|GetCameraBoom)) 3e+02 _returnvalue 1e+01)))))

(event Custom|Sequence_2
  ;[1 1 1] Sequence 2
)

(event Custom|Sequence_3
  ;[1 1 1] Sequence 3
)

(event Custom|Sequence_4
  ;[1 1 1] Sequence 4
)

(event Custom|Sequence_5
  ;[1 1 1] Sequence 5
)

(event Custom|Sequence_6
  ;[1 1 1] Sequence 6
)

(event Custom|Sequence_7)

(event EventTick
  (params (DeltaSeconds :type Float%20%28single-precision%29))
  (bind _charactermovement (Variables|Character|GetCharacterMovement))
  (Utilities|FlowControl|Sequence
    (:then_0
      (CallFunction|Sequence0)
      (CallFunction|Sequence1 :!label _label)
      (CallFunction|Sequence2 :!label _label_2)
      (CallFunction|Sequence3 :!label _label_3)
      (CallFunction|Sequence4 :!label _label_4)
      (CallFunction|Sequence5 :!label _label_5)
      (CallFunction|Sequence6 :!label _label_6))
    (:then_1
      (goto _label))
    (:then_2
      (goto _label_2))
    (:then_3
      (goto _label_3))
    (:then_4
      (goto _label_4))
    (:then_5
      (goto _label_5))
    (:then_6
      (goto _label_6))
    (:then_7
      _))
  (CallFunction|Sequence7)
  (if true
    (Variables|Default|SetIsRunning false)
    (Variables|/Script/Engine.CharacterMovementComponent|SetbOrientRotationToMovement _charactermovement false)
    (Variables|/Script/Engine.CharacterMovementComponent|SetMaxWalkSpeed _charactermovement 3e+02)))

(event Input|AxisEvents|InputAxisRollForward
  (params (AxisValue :type Float%20%28single-precision%29))
  (Variables|Default|SetMoveForwardAxis AxisValue))

(event Input|AxisEvents|InputAxisRollRight
  (params (AxisValue :type Float%20%28single-precision%29))
  (Variables|Default|SetMoveRightAxis AxisValue))

(event Input|AxisEvents|InputAxisLookUp
  (params (AxisValue :type Float%20%28single-precision%29))
  (Pawn|Input|AddControllerPitchInput AxisValue))

(event Input|AxisEvents|InputAxisTurn
  (params (AxisValue :type Float%20%28single-precision%29))
  (Pawn|Input|AddControllerYawInput AxisValue))

(event Input|AxisEvents|InputAxisMoveForward
  (params (AxisValue :type Float%20%28single-precision%29))
  (Pawn|Input|AddMovementInput (Math|Vector|GetForwardVector (Math|Rotator|MakeRotator 0.0 0.0 (.Yaw (Math|Rotator|BreakRotator (Pawn|GetControlRotation :!class /Script/Engine.Pawn))))) AxisValue false))

(event Input|AxisEvents|InputAxisMoveRight
  (params (AxisValue :type Float%20%28single-precision%29))
  (Pawn|Input|AddMovementInput (Math|Vector|GetRightVector (Math|Rotator|MakeRotator 0.0 0.0 (.Yaw (Math|Rotator|BreakRotator (Pawn|GetControlRotation :!class /Script/Engine.Pawn))))) AxisValue false))

(event Input|KeyboardEvents|SpaceBar
  (params (Key :type Key%20Structure :default "None"))
  ;[1 1 1] Space bar Process
)

(fn ConstructionScript
  (Variables|Default|SetHealthValue 1.0)
  (Variables|Default|SetEnergyValue 1.0)
  (bind _returnvalue (Actor|GetActorOfClass "/Script/Warriors.WarriorsCharacter"))
  (Variables|Default|SetEnemyCharacter _returnvalue))

(fn BPIsMoveSituation
  (if (or (Variables|Default|GetIsAttacking) (Variables|Default|Get%20IsPlayedAttackStateSwitch))
    (return false)
    (else
      (return false))))