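; Viking combat character, set against the Knight as its enemy, with sword attacks, stamina and health.
; Tick updates running and rolling stamina and feeds a screen status bar and health bar widget.
; Left click drives a single combo montage with buffered input, while collision events toggle the sword capsule that applies damage on overlap.
; Damage plays a hit reaction or flags death in ABP_Viking, and parries play a guard-break montage.
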(event OnComponentBeginOverlap(SwordCapsuleComponent)
  (params (OverlappedComponent :type Primitive%20Component%20Object%20Reference) (OtherActor :type Actor%20Object%20Reference) (OtherComp :type Primitive%20Component%20Object%20Reference) (OtherBodyIndex :type Integer) (bFromSweep :type Boolean) (SweepResult :type Hit%20Result%20Structure%20%28by%20ref%29))
  (if (!= OtherActor self)
    (Development|PrintString (Utilities|GetDisplayName OtherActor))
    (Game|Damage|ApplyDamage OtherActor 0.2 0 self)))

(event Custom|ParriedByEnemy
  (Animation|PlayAnimMontage "/Game/Animations/AM_Knight_GuardBreaked.AM_Knight_GuardBreaked" 1.0 "None"))

(event Custom|OnCollEnd_Attack
  (Collision|SetCollisionEnabled (Variables|Default|GetSwordCapsuleComponent) "NoCollision"))

(event Custom|OnCollStart_Attack
  (Collision|SetCollisionEnabled (Variables|Default|GetSwordCapsuleComponent) "QueryAndPhysics"))

(event EventBeginPlay
  (bind _returnvalue (UserInterface|CreateWidget "/Game/UI/Gameplay/UI_CharacterStatusBar.UI_CharacterStatusBar_C"))
  (Variables|Default|SetCharacterStatusBar _returnvalue)
  (UserInterface|Viewport|AddtoViewport _returnvalue 0)
  (Variables|Default|SetStamina 1.0)
  (Variables|Default|SetHealth 1.0))

(event EventTick
  (params (DeltaSeconds :type Float%20%28single-precision%29))
  (|StaminaSystem)
  (Progress|SetPercent (Variables|Default|GetHealthBar (.CharacterStatusBar (Variables|Default|GetCharacterStatusBar))) (Variables|Default|GetHealth))
  (bind _asui_enemy_health_bar (Utilities|Casting|CastTo (UserInterface|GetUserWidgetObject (Variables|Default|GetHealthBarWidget))))
  (Progress|SetPercent (Variables|Default|GetHealthBar _asui_enemy_health_bar) (Variables|Default|GetHealth))
  (if (Math|Boolean|NORBoolean (Class|AnimInstance|IsAnyMontagePlaying (Components|SkeletalMesh|GetAnimInstance (Variables|Character|GetMesh))) (Variables|Default|GetIsDead))
    _))

(event Game|Damage|EventAnyDamage
  (params (Damage :type Float%20%28single-precision%29) (DamageType :type Damage%20Type%20Object%20Reference) (InstigatedBy :type Controller%20Object%20Reference) (DamageCauser :type Actor%20Object%20Reference))
  (bind _output_get (Variables|Default|SetHealth (- (Variables|Default|GetHealth) Damage)))
  (if (>= _output_get 0.1)
    (Animation|PlayAnimMontage "/Game/Animations/AM_Knight_HitByEnemy.AM_Knight_HitByEnemy" 1.0 "None")
    (else
      (Variables|Default|SetIsDead true)
      (bind _asabp_viking (Utilities|Casting|CastToABP_Viking (Components|SkeletalMesh|GetAnimInstance (Variables|Character|GetMesh))))
      (Variables|/Game/Animations/ABP_Viking.ABP_Viking_C|SetIsDead _asabp_viking true))))

(event Input|MouseEvents|LeftMouseButton
  (params (Key :type Key%20Structure :default "None"))
  (:Pressed
    (|AttackSystem)))

(fn ConstructionScript
  (Variables|Default|SetHealth 1.0)
  (Variables|Default|SetStamina 1.0)
  (Class|WarriorsCharacter|SetEnemyCharacter "/Game/Blueprints/Characters/1_Knight.1_Knight_C"))

(event Input|KeyboardEvents|SpaceBar
  (params (Key :type Key%20Structure))
  (:Pressed
    (if (not (Variables|Default|GetbIsRolling))
      (if (< 0.25 (Variables|Default|GetStamina))
        (Variables|Default|SetRollStartedTime (Utilities|Time|GetTimeSeconds))
        (Variables|Default|SetStamina (- (Variables|Default|GetStamina) 0.25))
        (Variables|Default|SetbIsRolling true)))))

(event Custom|AttackEnd
  (Variables|Default|SetSaveAttack false)
  (Variables|Default|SetIsAttacking false)
  (return))

(event Custom|ResetCombo
  (if (Variables|Default|GetSaveAttack)
    (Variables|Default|SetSaveAttack false)
    (else
      (Variables|Default|SetSaveAttack false)
      (Variables|Default|SetIsAttacking false)
      (Animation|StopAnimMontage "/Game/Animations/AM_Knight_Attack.AM_Knight_Attack")))
  (return))