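; Game instance that owns front-end menus and multiplayer session flow, opening the main menu or, without saved player settings, the options menu.
; Events create widgets, caching most for reuse.
; Hosting creates an advanced session with a server name, then opens Warriors_Lobby as listen server; joining and destroying sessions are also handled.
; Session failures and client network errors reach an error dialog; the travel-error branch is hard-wired never to display.
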(event Custom|ShowMainMenu
  (bind _returnvalue (Game|GetPlayerController 0))
  ;[1 1 1] Show MainMenu and Mouse cursor
  (Variables|Widget|GetMainMenuWB ; Has Main Menu already been created
    (:then
      _)
    (:else
      (bind _returnvalue_2 (UserInterface|CreateWidget "/Game/UI/MainMenu/MainMenu.MainMenu_C" _returnvalue))
      (Variables|Widget|SetMainMenuWB _returnvalue_2)))
  (UserInterface|Viewport|AddtoViewport (Variables|Widget|GetMainMenuWB) 0)
  (Variables|/Script/Engine.PlayerController|SetbShowMouseCursor _returnvalue true))

(event Custom|ShowHostMenu
  ;[1 1 1] Host Game Menu
  (Variables|Widget|GetHostMenuWB
    (:then
      _)
    (:else
      (bind _returnvalue (UserInterface|CreateWidget "/Game/UI/MainMenu/HostMenu.HostMenu_C" (Game|GetPlayerController 0)))
      (Variables|Widget|SetHostMenuWB _returnvalue)))
  (UserInterface|Viewport|AddtoViewport (Variables|Widget|GetHostMenuWB) 0))

(event Custom|ShowServerMenu
  ;[1 1 1] Show Server Menu
  (bind _returnvalue (UserInterface|CreateWidget "/Game/UI/MainMenu/ServerMenu.ServerMenu_C" (Game|GetPlayerController 0)))
  (UserInterface|Viewport|AddtoViewport _returnvalue 0))

(event Custom|ShowOptionMenu
  ;[1 1 1] Show Option Menu
  (Variables|Widget|GetOptionMenuWB
    (:then
      _)
    (:else
      (bind _returnvalue (UserInterface|CreateWidget "/Game/UI/MainMenu/OptionsMenu.OptionsMenu_C" (Game|GetPlayerController 0)))
      (Variables|Widget|SetOptionMenuWB _returnvalue)))
  (UserInterface|Viewport|AddtoViewport (Variables|Widget|GetOptionMenuWB) 0))

(event Custom|LaunchLobby
  (params (NunberOfPlayer :type Integer) (EnableLAN :type Boolean) (ServerName :type Text))
  ;[1 1 1] Launch Lobby with host setting
  (Variables|ServerSetting|SetMaxPlayer NunberOfPlayer)
  (bind _output_get (Variables|ServerSetting|SetServerName ServerName))
  (CallFunction|ShowLoadingScreen)
  (|AdvancedSession (Utilities|Array|MakeArray (Class|AdvancedSessionsLibrary|MakeLiteralSessionPropertyString "ServerName" (Utilities|String|ToString(Text) _output_get)) "") (Game|GetPlayerController 0) (Variables|ServerSetting|GetMaxPlayer) 0 EnableLAN true false true true false false false true
    (:OnSuccess
      (Game|OpenLevel(byName) "Warriors_Lobby" false "listen"))
    (:OnFailure
      (Utilities|DisplayErrorMessage "Faild Create Session"))))

(event Custom|ShowLoadingScreen
  ;[1 1 1] Show Loading Screen
  (Variables|Widget|GetLoadingScreenWB
    (:then
      _)
    (:else
      (bind _returnvalue (UserInterface|CreateWidget "/Game/UI/AllLevels/LoadingScreen.LoadingScreen_C" (Game|GetPlayerController 0)))
      (Variables|Widget|SetLoadingScreenWB _returnvalue)))
  (UserInterface|Viewport|AddtoViewport (Variables|Widget|GetLoadingScreenWB) 0))

(event Custom|JoinServer
  (params (Session%20to%20Join :type Blueprint%20Session%20Result%20Structure))
  ;[1 1 1] Join Server and Call Server Menu
  (CallFunction|ShowLoadingScreen)
  (|JoinSession (Game|GetPlayerController 0) Session%20to%20Join
    (:OnFailure
      (Utilities|DisplayErrorMessage "Faild Join Session"))))

(event Custom|DestroySessionCaller
  (params (Player%20Controller :type Player%20Controller%20Object%20Reference))
  ;[1 1 1] Destroy Session when called
  (|DestroySession Player%20Controller))

(event Custom|SaveGameCheck
  ;[1 1 1] Check Save Game
  (SaveGame|DoesSaveGameExist (Variables|Default|GetPlayer_Setting_Save))
  (if true
    (CallFunction|ShowMainMenu)
    (Variables|Default|SetIsCreateSaveFile true)
    (else
      (CallFunction|ShowOptionMenu)
      (Variables|/Script/Engine.PlayerController|SetbShowMouseCursor (Game|GetPlayerController 0) true))))

(event Custom|ShowSessionMenu
  ;[1 1 1] Show Session Menu
  (bind _returnvalue (UserInterface|CreateWidget "/Game/UI/MainMenu/Server_ListMenu.Server_ListMenu_C" (Game|GetPlayerController 0)))
  (UserInterface|Viewport|AddtoViewport _returnvalue 0))

(event EventHandleNetworkError
  (params (FailureType :type ENetworkFailure%20Enum :default "NetDriverAlreadyExists") (bIsServer :type Boolean))
  ;[1 1 1] Network Error Message Output
  (if (not bIsServer)
    (Utilities|DisplayErrorMessage (CallFunction|NetworkErrortoString FailureType))))

(event EventHandleTravelError
  (params (FailureType :type ETravelFailure%20Enum :default "NoLevel"))
  ;[1 1 1] Travel Error Message Output
  (if (not true)
    (Utilities|DisplayErrorMessage (CallFunction|TravelErrortoString FailureType))))

(fn OnRepServerName)

(fn NetworkErrortoString
  (params (FailureType :type ENetworkFailure%20Enum :default "NetDriverAlreadyExists"))
  (switch Utilities|FlowControl|Switch|SwitchonENetworkFailure FailureType
    (:NetDriverAlreadyExists
      (Variables|Default|SetErrorSting "Error_Lost_Connection_to_Host" :!label _label))
    (:NetDriverCreateFailure
      (goto _label))
    (:NetDriverListenFailure
      (goto _label))
    (:ConnectionLost
      (goto _label))
    (:ConnectionTimeout
      (Variables|Default|SetErrorSting "Error_Connection_Time_Out"))
    (:FailureReceived
      (goto _label))
    (:OutdatedClient
      (goto _label))
    (:OutdatedServer
      (goto _label))
    (:PendingConnectionFailure
      (goto _label))
    (:NetGuidMismatch
      (goto _label))
    (:NetChecksumMismatch
      (goto _label)))
  (return (Variables|Default|GetErrorSting)))

(fn TravelErrortoString
  (params (FailureType :type ETravelFailure%20Enum :default "NoLevel"))
  (return (Utilities|String|Append "Error_Failed_to_Travel" (Utilities|String|EnumtoString FailureType))))